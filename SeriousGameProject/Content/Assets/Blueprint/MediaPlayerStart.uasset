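; Cutscene actor that plays the first "Look Away" cutscene video when play begins.
; On BeginPlay it shows a plane, activates a separate cutscene sound component and opens the video source on a media player.
; Player move input is ignored during a hard-coded delay of 56 seconds, rather than waiting on a media-end event, then restored before the actor destroys itself.
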(event `self.ReceiveBeginPlay`
  (bind _returnvalue (`GameplayStatics.GetPlayerController` 0))
  (`SceneComponent.SetVisibility` (`self.Shape_Plane`) true false)
  (`ActorComponent.Activate` (`self.LookAwayCutscene_Sound`) false)
  (`MediaPlayer.OpenSource` (`self.MediaPlayer`) "/Game/Movies/02_Look_Away_Cutscene_1.02_Look_Away_Cutscene_1")
  (`Controller.SetIgnoreMoveInput` _returnvalue true)
  (`KismetSystemLibrary.Delay` 56.0)
  (`Controller.SetIgnoreMoveInput` _returnvalue false)
  (`self.K2_DestroyActor`))

(fn `UserConstructionScript`)