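; bp_Start runs a timed intro camera sequence when play begins.
; It sets AIStop on the FirstPersonCharacter, blocks move input and cuts to the actor that owns its Camera.
; After a delay it blends back to the saved view target and restores movement.
; After a second delay it sets PlayerIsViewer, clears AIStop and calls CallEvnViewerChange.
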(event `self.ReceiveBeginPlay`
  (bind _returnvalue (`GameplayStatics.GetPlayerController` 0))
  (bind _returnvalue_2 (`GameplayStatics.GetPlayerController` 0))
  (`|ExecutionSequence`
    (:`then_0`
      (bind _asfirst_person_character (cast `/Game/FirstPersonBP/Blueprints/FirstPersonCharacter` (`GameplayStatics.GetPlayerPawn` 0)))
      (set `/Game/FirstPersonBP/Blueprints/FirstPersonCharacter.AIStop!` true _asfirst_person_character))
    (:`then_1`
      (set `self.PlayerCam` (`Controller.GetViewTarget` (`GameplayStatics.GetPlayerController` 0)))
      (`Controller.SetIgnoreMoveInput` _returnvalue_2 true)
      (`PlayerController.SetViewTargetWithBlend` _returnvalue_2 (`ActorComponent.GetOwner` (`self.Camera`)) 0.0 "VTBlend_EaseInOut" 0.8 false)
      ;[1 1 1] Adding Specific State here
      (`KismetSystemLibrary.Delay` 5.0)
      (`PlayerController.SetViewTargetWithBlend` _returnvalue (`self.PlayerCam`) 0.2 "VTBlend_EaseInOut" 0.8 false)
      (`Controller.SetIgnoreMoveInput` _returnvalue false)
      ;[1 1 1] Adding Specific State here
      (`KismetSystemLibrary.Delay` 5.0)
      (set `self.PlayerIsViewer` true)
      (bind _asfirst_person_character_2 (cast `/Game/FirstPersonBP/Blueprints/FirstPersonCharacter` (`GameplayStatics.GetPlayerPawn` 0)))
      (set `/Game/FirstPersonBP/Blueprints/FirstPersonCharacter.AIStop!` false _asfirst_person_character_2)
      (`self.evn_ViewerChange`))))

(fn `UserConstructionScript`)