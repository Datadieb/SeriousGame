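; Hideout actor that lets the first-person player hide inside it and view from its own camera.
; A box overlap marks the player as in range, while a delayed Tick polls the character's use button.
; Two mutually resetting DoOnce gates alternate entering and leaving based on the character's Hidden flag.
; Each switch toggles that flag and move input, blending between the hideout camera and the view target saved at BeginPlay.
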(event `self.ReceiveBeginPlay`
  (set `self.PlayerCam` (`Controller.GetViewTarget` (`GameplayStatics.GetPlayerController` 0))))

(event `self.Box.OnComponentBeginOverlap`
  (params (OverlappedComponent :type "PrimitiveComponent Object Reference") (OtherActor :type "Actor Object Reference") (OtherComp :type "PrimitiveComponent Object Reference") (OtherBodyIndex :type Integer) (bFromSweep :type Boolean) (SweepResult :type "HitResult Structure (by ref)"))
  (if (== OtherActor (`GameplayStatics.GetPlayerCharacter` 0))
    (set `self.Triggered?` true)))

(event `self.Box.OnComponentEndOverlap`
  (params (OverlappedComponent :type "PrimitiveComponent Object Reference") (OtherActor :type "Actor Object Reference") (OtherComp :type "PrimitiveComponent Object Reference") (OtherBodyIndex :type Integer))
  (if (== (`GameplayStatics.GetPlayerCharacter` 0) OtherActor)
    (set `self.Triggered?` false)))

(event `self.ReceiveTick`
  (params (DeltaSeconds :type "Float (single-precision)"))
  (bind _returnvalue (`GameplayStatics.GetPlayerController` 0))
  (bind _returnvalue_2 (`GameplayStatics.GetPlayerController` 0))
  (`KismetSystemLibrary.Delay` 0.2)
  (bind _asfirst_person_character (cast `/Game/FirstPersonBP/Blueprints/FirstPersonCharacter` (`GameplayStatics.GetPlayerPawn` 0)))
  (if (`/Game/FirstPersonBP/Blueprints/FirstPersonCharacter.Use Button Pressed` _asfirst_person_character)
    (if (`self.Triggered?`)
      (if (`/Game/FirstPersonBP/Blueprints/FirstPersonCharacter.Hidden` _asfirst_person_character)
        (`/Engine/EditorBlueprintResources/StandardMacros.DoOnce` false :!label _label
          (:`Completed`
            (`PlayerController.SetViewTargetWithBlend` _returnvalue (`self.PlayerCam`) 0.2 "VTBlend_EaseInOut" 0.8 false)
            (set `/Game/FirstPersonBP/Blueprints/FirstPersonCharacter.Hidden` false _asfirst_person_character)
            (`Controller.SetIgnoreMoveInput` _returnvalue false)
            (goto _label_2 :!via `Reset`)))
        (else
          (`/Engine/EditorBlueprintResources/StandardMacros.DoOnce` false :!label _label_2
            (:`Completed`
              (set `/Game/FirstPersonBP/Blueprints/FirstPersonCharacter.Hidden` true _asfirst_person_character)
              (`Controller.SetIgnoreMoveInput` _returnvalue_2 true)
              (`PlayerController.SetViewTargetWithBlend` _returnvalue_2 (`ActorComponent.GetOwner` (`self.Camera`)) 0.2 "VTBlend_EaseInOut" 0.8 false)
              (goto _label :!via `Reset`))))))))

(fn `UserConstructionScript`)