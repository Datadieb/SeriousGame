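; Window-jump Blueprint with a trigger volume that teleports on overlap and plays a brief camera transition.
; The overlap check compares the other actor to the player controller itself, and the teleport moves that controller to the Sphere component's location.
; It then blends the view to this actor with a camera shake, and after a short delay blends to the stored PlayerCameraManager as view target.
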(event `self.Trigger.OnComponentBeginOverlap`
  (params (OverlappedComponent :type "PrimitiveComponent Object Reference") (OtherActor :type "Actor Object Reference") (OtherComp :type "PrimitiveComponent Object Reference") (OtherBodyIndex :type Integer) (bFromSweep :type Boolean) (SweepResult :type "HitResult Structure (by ref)"))
  (bind _returnvalue (`GameplayStatics.GetPlayerController` 0))
  (bind _returnvalue_2 (`GameplayStatics.GetPlayerController` 0))
  (set `self.IntialCam` (`PlayerController.PlayerCameraManager` _returnvalue))
  (if (== _returnvalue OtherActor)
    (`self.K2_TeleportTo` :`self` (`GameplayStatics.GetPlayerController` 0) :`DestLocation` (`SceneComponent.K2_GetComponentLocation` (`self.Sphere`)))
    (`PlayerController.SetViewTargetWithBlend` _returnvalue self 1.0 "VTBlend_Linear" 0.0 false)
    (`PlayerController.ClientStartCameraShake` :`self` _returnvalue_2)
    (`KismetSystemLibrary.Delay` 1.0)
    (`PlayerController.SetViewTargetWithBlend` _returnvalue_2 (`self.IntialCam`) 1.0 "VTBlend_Linear" 0.0 false)))

(fn `UserConstructionScript`)