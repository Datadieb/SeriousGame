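; Background extra character that takes its mesh from ChooseCharacter and wanders endlessly between Statisten_TargetPoint actors.
; It picks a random point, moves there with AIMoveTo, then waits briefly after success or failure before choosing again.
; After issuing a move, it repicks if a randomly drawn point is too close.
; The stored target, destination and distance check each use separate random draws, so they can differ.
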(event `self.ReceiveBeginPlay`
  (`|ExecutionSequence`
    (:`then_0`
      (`SkinnedMeshComponent.SetSkinnedAssetAndUpdate` (`self.Mesh`) (`self.ChooseCharacter`) false))
    (:`then_1`
      (bind _outactors (`GameplayStatics.GetAllActorsOfClass` "/Game/Assets/KI/TargetPointClass/Statisten_TargetPoint.Statisten_TargetPoint_C" :!label _label))
      (bind _item (`KismetArrayLibrary.Array_Get` _outactors (`KismetMathLibrary.RandomIntegerInRange` 0 (`KismetArrayLibrary.Array_LastIndex` _outactors))))
      (set `self.CurrentTargetPoint` _item :!label _label_2)
      (bind _returnvalue (`self.K2_GetActorLocation` _item))
      (set `self.TargetPoint` _returnvalue)
      (`|ExecutionSequence`
        (:`then_0`
          (`|AIMoveTo` self (`self.TargetPoint`)
            (:`OnSuccess`
              _)
            (:`OnFail`
              _))
          (`KismetSystemLibrary.Delay` 5.0)
          (`self.Targetpoint reached!_Event`))
        (:`then_1`
          (`/Engine/EditorBlueprintResources/StandardMacros.CompareFloat` (`KismetMathLibrary.VSize` (- (`self.K2_GetActorLocation` self) _returnvalue)) 250.0
            (:`<`
              (goto _label_2))))))))

(event `Targetpoint reached!_Event`
  (goto _label))

(fn `UserConstructionScript`)