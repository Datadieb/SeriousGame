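; One-shot toilet dialogue cutscene Blueprint, fired by the first overlap of its Trigger.
; If the player overlaps, it calls ToiletEventStarted, cuts to the Camera's owner and plays a timed, colour-coded Stewart, Marc and Alicia exchange in the ToiletDialogue widget.
; It then blends back to the saved view, calls ToiletEventEnded and hides DialogueEvent.
; DoOnce and showing DialogueEvent precede the player check, so another actor can consume the event.
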(event `self.Trigger.OnComponentBeginOverlap`
  (params (OverlappedComponent :type "PrimitiveComponent Object Reference") (OtherActor :type "Actor Object Reference") (OtherComp :type "PrimitiveComponent Object Reference") (OtherBodyIndex :type Integer) (bFromSweep :type Boolean) (SweepResult :type "HitResult Structure (by ref)"))
  (bind _text (`self.Text`))
  (bind _text_2 (`self.Text`))
  (bind _text_3 (`self.Text`))
  (bind _text_4 (`self.Text`))
  (bind _text_5 (`self.Text`))
  (bind _text_6 (`self.Text`))
  (bind _text_7 (`self.Text`))
  (`/Engine/EditorBlueprintResources/StandardMacros.DoOnce` false
    (:`Completed`
      (`SceneComponent.SetVisibility` (`self.DialogueEvent`) true false)
      (set `self.IntialCam` (`Controller.GetViewTarget` (`GameplayStatics.GetPlayerController` 0)))
      (if (== OtherActor (`GameplayStatics.GetPlayerCharacter` 0))
        (`self.ToiletEventStarted`)
        (`PlayerController.SetViewTargetWithBlend` (`GameplayStatics.GetPlayerController` 0) (`ActorComponent.GetOwner` (`self.Camera`)) 0.0 "VTBlend_Linear" 0.0 false)
        (bind _foundwidgets (`WidgetBlueprintLibrary.GetAllWidgetsOfClass` "/Game/Assets/UI/UMG/ToiletDialogue.ToiletDialogue_C" false))
        (bind _astoilet_dialogue (cast `/Game/Assets/UI/UMG/ToiletDialogue` (`KismetArrayLibrary.Array_Get` _foundwidgets)))
        (bind _output_get (set `self.Text` (`/Game/Assets/UI/UMG/ToiletDialogue.DialogueTime` _astoilet_dialogue)))
        (`|ExecutionSequence`
          (:`then_0`
            (`TextBlock.SetColorAndOpacity` _text (`self.StewartColor`))
            (`TextBlock.SetColorAndOpacity` _output_get (`self.StewartColor`)))
          (:`then_1`
            (`TextBlock.SetText` _text (`self.StewartText1`))
            (`TextBlock.SetText` _output_get (`self.StewartText1`))
            (`KismetSystemLibrary.Delay` (`self.TextSpeed`))
            (`|ExecutionSequence`
              (:`then_0`
                (`TextBlock.SetColorAndOpacity` _text_2 (`self.MarcColor`)))
              (:`then_1`
                (`TextBlock.SetText` _text_2 (`self.MarcText1`))
                (`KismetSystemLibrary.Delay` (`self.TextSpeed`))
                (`|ExecutionSequence`
                  (:`then_0`
                    (`TextBlock.SetColorAndOpacity` _text_3 (`self.StewartColor`)))
                  (:`then_1`
                    (`TextBlock.SetText` _text_3 (`self.StewartText2`))
                    (`KismetSystemLibrary.Delay` (`self.TextSpeed`))
                    (`|ExecutionSequence`
                      (:`then_0`
                        (`TextBlock.SetColorAndOpacity` _text_4 (`self.AliciaColor`)))
                      (:`then_1`
                        (`TextBlock.SetText` _text_4 (`self.AliciaText1`))
                        (`KismetSystemLibrary.Delay` (`self.TextSpeed`))
                        (`|ExecutionSequence`
                          (:`then_0`
                            (`TextBlock.SetColorAndOpacity` _text_5 (`self.MarcColor`)))
                          (:`then_1`
                            (`TextBlock.SetText` _text_5 (`self.MarcText2`))
                            (`KismetSystemLibrary.Delay` (`self.TextSpeed`))
                            (`|ExecutionSequence`
                              (:`then_0`
                                (`TextBlock.SetColorAndOpacity` _text_6 (`self.StewartColor`)))
                              (:`then_1`
                                (`TextBlock.SetText` _text_6 (`self.StewartText3`))
                                (`KismetSystemLibrary.Delay` (`self.TextSpeed`))
                                (`|ExecutionSequence`
                                  (:`then_0`
                                    (`TextBlock.SetColorAndOpacity` _text_7 (`self.AliciaColor`)))
                                  (:`then_1`
                                    (`TextBlock.SetText` _text_7 (`self.AliciaText2`))
                                    (`KismetSystemLibrary.Delay` (`self.TextSpeed`))
                                    (`PlayerController.SetViewTargetWithBlend` (`GameplayStatics.GetPlayerController` 0) (`self.IntialCam`) 2.0 "VTBlend_Linear" 0.0 false)
                                    (`self.ToiletEventEnded`)
                                    (`SceneComponent.SetVisibility` (`self.DialogueEvent`) false false)))))))))))))))))))

(fn `UserConstructionScript`)