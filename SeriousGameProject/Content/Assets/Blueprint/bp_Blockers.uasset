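; Blocker actor that removes its Collider once the game reaches a specified phase.
; On BeginPlay it binds an event to the phase change dispatcher of FirstPersonGameMode.
; When the game mode's Phase matches the WelchePhase variable, a DoOnce gate destroys the Collider component.
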(event `self.ReceiveBeginPlay`
  (bind _asfirst_person_game_mode (cast `/Game/FirstPersonBP/Blueprints/FirstPersonGameMode` (`GameplayStatics.GetGameMode`)))
  (add `/Game/FirstPersonBP/Blueprints/FirstPersonGameMode.PhaseChange` _asfirst_person_game_mode (delegate `Phase0Ended_Event`)))

(event `Phase0Ended_Event`
  (if (== (`/Game/FirstPersonBP/Blueprints/FirstPersonGameMode.Phase` (stale `self.ReceiveBeginPlay` _asfirst_person_game_mode)) (`self.WelchePhase?`))
    (`/Engine/EditorBlueprintResources/StandardMacros.DoOnce` false
      (:`Completed`
        (`ActorComponent.K2_DestroyComponent` (`self.Collider`))))))

(fn `UserConstructionScript`)