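; Main menu actor that hosts the UMG_MainMenu widget in a widget component and has its own camera view.
; On BeginPlay it sets game-only input and binds the widget's settings-pressed event, which hands control to the referenced Settings object through TakeInputControl.
; TakeInputControlMM blends the player's view to this actor's Camera with an ease-in-out transition.
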(event `self.ReceiveBeginPlay`
  (`WidgetBlueprintLibrary.SetInputMode_GameOnly` (`GameplayStatics.GetPlayerController` 0))
  (bind _asumg_main_menu (cast `/Game/HUD/Menus/MainMenu/UMG_MainMenu` (`WidgetComponent.GetUserWidgetObject` (`self.Menu`))))
  (add `/Game/HUD/Menus/MainMenu/UMG_MainMenu.OnSettingsPressed` _asumg_main_menu (delegate `OnSettingsPressed_Event`)))

(event `OnSettingsPressed_Event`
  (`/Game/HUD/Menus/MainMenu/BP_SettingsMenu.Take Input Control` (`self.Settings`)))

(fn `Take Input Control MM`
  (`PlayerController.SetViewTargetWithBlend` (`GameplayStatics.GetPlayerController` 0) (`self.Camera`) 2.0 "VTBlend_EaseInOut" 1.3 false))

(fn `UserConstructionScript`)