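; BP_SettingsMenu is an actor that presents the settings screen of the main menu through a widget component with its own camera.
; On BeginPlay it casts the widget to UMG_Settings and binds its back-pressed event, which hands input control back to the main menu.
; TakeInputControl eases the player's view over to this menu's camera with a timed blend, so menu switches play as camera moves.
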(event `self.ReceiveBeginPlay`
  (bind _asumg_settings (cast `/Game/HUD/Menus/MainMenu/UMG_Settings` (`WidgetComponent.GetUserWidgetObject` (`self.Menu`))))
  (add `/Game/HUD/Menus/MainMenu/UMG_Settings.OnBackPressed` _asumg_settings (delegate `OnBackPressed_Event`)))

(event `OnBackPressed_Event`
  (`/Game/HUD/Menus/MainMenu/BP_Mainmenu.Take Input Control MM` (`self.MainMenu`)))

(fn `Take Input Control`
  (`PlayerController.SetViewTargetWithBlend` (`GameplayStatics.GetPlayerController` 0) (`self.Camera`) 2.0 "VTBlend_EaseInOut" 1.3 false))

(fn `UserConstructionScript`)